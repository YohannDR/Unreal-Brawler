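; Behavior Tree task that plays Kassadin's attack for an AI-controlled BP_Kassadin.
; It clears the BBDCanMove blackboard key, then picks the W-empowered or basic attack montage based on WActive.
; The W montage, on completion or interruption, consumes WActive and starts its cooldown timer before restoring movement and finishing successfully.
; The basic montage restores movement and finishes only on completion, with no interruption handling.
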(event `self.ReceiveExecuteAI`
  (params (OwnerController :type "AIController Object Reference") (ControlledPawn :type "Pawn Object Reference"))
  (bind _asbp_kassadin (cast `/Game/Content/Blueprint/Kassadin/BP_Kassadin` ControlledPawn))
  (`BTFunctionLibrary.SetBlackboardValueAsBool` (`self.BBDCanMove`))
  (if (`/Game/Content/Blueprint/Kassadin/BP_Kassadin.WActive` _asbp_kassadin)
    (bind _mesh (`Character.Mesh` _asbp_kassadin))
    (`|PlayMontage` _mesh "/Game/Content/Animation/Kassadin/Montage/AM_KassadinAttackW.AM_KassadinAttackW"
      (:`OnCompleted`
        _)
      (:`OnInterrupted`
        _))
    (set `/Game/Content/Blueprint/Kassadin/BP_Kassadin.WActive` false _asbp_kassadin)
    (set `/Game/Content/Blueprint/Kassadin/BP_Kassadin.WTimer` (`/Game/Content/Blueprint/Kassadin/BP_Kassadin.WCooldown` _asbp_kassadin) _asbp_kassadin)
    (else
      (`|PlayMontage` _mesh "/Game/Content/Animation/Kassadin/Montage/AM_KassadinAttack.AM_KassadinAttack"
        (:`OnCompleted`
          _))))
  (`BTFunctionLibrary.SetBlackboardValueAsBool` (`self.BBDCanMove`) true)
  (`self.FinishExecute` true))