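; AI controller for the Kassadin enemy, running its behavior tree on possess and feeding it combat state.
; On the first tick it stores player 0 as the target on the blackboard and pawn, and enables movement.
; Every tick it refreshes attack range and R-usage flags from the pawn, and clears the blackboard target when the player dies.
; A remapped facing dot product flags when the pawn should rotate toward the target.
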(event `self.ReceivePossess`
  (params (PossessedPawn :type "Pawn Object Reference"))
  ;[1 1 1] Start behavior tree
  (`self.RunBehaviorTree` "/Game/Content/Blueprint/Kassadin/BT_Kassadin.BT_Kassadin"))

(event `self.ReceiveTick`
  (params (DeltaSeconds :type "Float (single-precision)"))
  (bind _returnvalue (`self.K2_GetPawn`))
  (`|ExecutionSequence`
    (:`then_0`
      (`/Engine/EditorBlueprintResources/StandardMacros.DoOnce` false
        (:`Completed`
          ;[1 1 1] On first update
          (`|ExecutionSequence`
            (:`then_0`
              ;;[1 1 1] Save player instance as target
              (bind _output_get (set `self.Target` (`GameplayStatics.GetPlayerCharacter` 0)))
              (`BlackboardComponent.SetValueAsObject` (`AIBlueprintHelperLibrary.GetBlackboard` null) "Target" _output_get)
              (bind _asbp_kassadin (cast `/Game/Content/Blueprint/Kassadin/BP_Kassadin` (`self.K2_GetPawn`)))
              (set `/Game/Content/Blueprint/Kassadin/BP_Kassadin.Target` (`self.Target`) _asbp_kassadin))
            (:`then_1`
              ;;[1 1 1] Set CanMove to true
              (`BlackboardComponent.SetValueAsBool` (`AIBlueprintHelperLibrary.GetBlackboard` null) "CanMove" true))))))
    (:`then_1`
      (`|ExecutionSequence`
        (:`then_0`
          ;[1 1 1] Update target in range state
          (bind _asbp_kassadin_2 (cast `/Game/Content/Blueprint/Kassadin/BP_Kassadin` (`self.K2_GetPawn`)))
          (`BlackboardComponent.SetValueAsBool` (`AIBlueprintHelperLibrary.GetBlackboard` null) "TargetInAttackRange" (`/Game/Content/Blueprint/Kassadin/BP_Kassadin.IsTargetInRange` _asbp_kassadin_2)))
        (:`then_1`
          ;[1 1 1] Set target to null if dead
          (bind _asplayer_cpp (cast `PlayerCPP` (`self.Target`)))
          (if (`/Game/Content/Blueprint/Player/BP_Player.Dead` _asplayer_cpp)
            (`BlackboardComponent.SetValueAsObject` (`AIBlueprintHelperLibrary.GetBlackboard` null) "Target" null)))
        (:`then_2`
          ;[1 1 1] Update whether to use R
          (bind _asbp_kassadin_3 (cast `/Game/Content/Blueprint/Kassadin/BP_Kassadin` (`self.K2_GetPawn`)))
          (`BlackboardComponent.SetValueAsBool` (`AIBlueprintHelperLibrary.GetBlackboard` null) "ShouldR" (`/Game/Content/Blueprint/Kassadin/BP_Kassadin.ShouldUseR` _asbp_kassadin_3)))
        (:`then_3`
          ;[1 1 1] Update whether to rotate towards the target
          (`BlackboardComponent.SetValueAsBool` (`AIBlueprintHelperLibrary.GetBlackboard` null) "ShouldRotateTowardsTarget" (< (/ (+ (`KismetMathLibrary.Dot_VectorVector` (`KismetMathLibrary.Normal` (- (`self.K2_GetActorLocation` (`self.Target`)) (`self.K2_GetActorLocation` _returnvalue))) (`KismetMathLibrary.Conv_RotatorToVector` (`self.K2_GetActorRotation` _returnvalue))) 1.0) 2.0) 0.9)))))))

(fn `UserConstructionScript`)