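; Behavior Tree task that moves the AI-controlled Kassadin toward its current target.
; On execute it runs an AI MoveTo on the pawn's Target, with an acceptance radius set to a fraction of its attack range, and finishes on success.
; Each tick it checks the ShouldR blackboard flag, stopping movement and finishing early when R can be used.
; A failed move has no finish path.
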(event `self.ReceiveTickAI`
  (params (OwnerController :type "AIController Object Reference") (ControlledPawn :type "Pawn Object Reference") (DeltaSeconds :type "Float (single-precision)"))
  ;[1 1 1] Stop movement if able to R
  (if (`BTFunctionLibrary.GetBlackboardValueAsBool` (`self.BBDShouldR`))
    (`Controller.StopMovement` OwnerController)
    (`self.FinishExecute` true)))

(event `self.ReceiveExecuteAI`
  (params (OwnerController :type "AIController Object Reference") (ControlledPawn :type "Pawn Object Reference"))
  ;[1 1 1] Move to target
  (bind _asbp_kassadin (cast `/Game/Content/Blueprint/Kassadin/BP_Kassadin` ControlledPawn))
  (`|AIMoveTo` _asbp_kassadin (0.0 0.0 0.0) (`/Game/Content/Blueprint/Kassadin/BP_Kassadin.Target` _asbp_kassadin) (* (`Enemy.AttackRange` _asbp_kassadin) 0.7)
    (:`OnSuccess`
      (`self.FinishExecute` true))))