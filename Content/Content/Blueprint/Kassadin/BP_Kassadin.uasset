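; Kassadin combat character that tracks a target, manages its W and R spell cooldowns, and fades out on death.
; Tick arms W with cover and glow visuals when ready, and flags R with a range-capped horizontal destination when the target is far enough.
; Damage values are chosen by matching substrings in the current animation's name.
; At zero health it plays a death animation and lowers dynamic-material opacity each frame until destroyed.
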(event `self.ReceiveTick`
  (params (DeltaSeconds :type "Float (single-precision)"))
  (bind _mesh (`self.Mesh`))
  (bind _returnvalue (not (`self.WActive`)))
  (`parent.ReceiveTick` DeltaSeconds)
  (if (`self.Dead`)
    ;[1 1 1] Death animation alpha
    (bind _output_get (set `self.DeathAnimationCurrentAlpha` (- (stale _output_get) (/ DeltaSeconds 4.8))))
    (for (_array_element _array_index) (`MeshComponent.GetMaterials` _mesh)
      (bind _returnvalue_2 (`PrimitiveComponent.CreateDynamicMaterialInstance` _mesh 0 _array_element "None"))
      (`MaterialInstanceDynamic.SetScalarParameterValue` _returnvalue_2 "Opacity" (`self.DeathAnimationCurrentAlpha`))
      (`PrimitiveComponent.SetMaterial` (`self.Mesh`) _array_index _returnvalue_2)
      (if (<= (`self.DeathAnimationCurrentAlpha`) 0.0)
        (`self.K2_DestroyActor`)))
    (else
      (`|ExecutionSequence`
        (:`then_0`
          ;[1 1 1] Decrease timers
          (bind _output_get_2 (set `self.WTimer` (- (stale _output_get_2) DeltaSeconds)))
          (bind _output_get_3 (set `self.RTimer` (- (stale _output_get_3) DeltaSeconds))))
        (:`then_1`
          ;[1 1 1] W spell
          (`|ExecutionSequence`
            (:`then_0`
              (if (and (<= (`self.WTimer`) 0.0) _returnvalue)
                (bind _output_get_4 (set `self.WActive` true))
                (`self.SetWVisible` _output_get_4)))
            (:`then_1`
              (if _returnvalue
                (`self.SetWVisible` false)))))
        (:`then_2`
          ;[1 1 1] R spell
          (bind _output_get_5 (set `self.ShouldUseR` (and (<= (`self.RTimer`) 0.0) (> (`self.TargetDistance`) (* (`self.RMaxDistance`) 0.5)))))
          (if _output_get_5
            (set `self.RDestinationLocation` (+ (* (`KismetMathLibrary.Normal` (`self.GetTargetDistance`)) (`KismetMathLibrary.FMin` (`self.TargetDistance`) (`self.RMaxDistance`))) (`self.K2_GetActorLocation`)))))
        (:`then_3`
          ;[1 1 1] Update target distance
          (set `self.TargetDistance` (`KismetMathLibrary.VSize` (`self.GetTargetDistance`))))))))

(event `self.OnDamageTaken`
  (params (DamageAmount :type "Float (single-precision)"))
  ;[1 1 1] Death
  (if (<= (`self.Health`) 0.0)
    (set `self.Dead` true)
    (`self.SetWVisible` false)
    (`SkeletalMeshComponent.PlayAnimation` (`self.Mesh`) "/Game/Content/Models/Kassadin/Animations/kassadin_skin05_death.kassadin_skin05_death" false)))

(fn `GetCurrentAnimationDamage`
  (returns (ReturnValue :type "Float (single-precision)"))
  (bind _returnvalue (`KismetStringLibrary.Conv_NameToString` (`self.GetCurrentAnimation`)))
  (if (`KismetStringLibrary.Contains` _returnvalue "strongAttack")
    (return (`self.WDamage`))
    (elif (`KismetStringLibrary.Contains` _returnvalue "dash")
      (return (`self.RDamage`))
      (elif (`KismetStringLibrary.Contains` _returnvalue "attack")
        (return (`self.AttackDamage`))
        (else
          (return 0.0))))))

(fn `GetTargetDistance`
  (returns (Distance :type "Vector Structure"))
  (bind (_returnvalue_x _returnvalue_y) (`KismetMathLibrary.BreakVector` (- (`self.K2_GetActorLocation` (`self.Target`)) (`self.K2_GetActorLocation`))))
  (return (`KismetMathLibrary.MakeVector` _returnvalue_x _returnvalue_y)))

(fn `IsTargetInRange`
  (returns (TargetInRange :type Boolean))
  (return (< (`self.TargetDistance`) (`self.AttackRange`))))

(fn `SetWVisible`
  (params (Visible :type Boolean))
  (`SceneComponent.SetVisibility` (`self.WCover`) Visible false)
  (`SceneComponent.SetVisibility` (`self.WGlow`) Visible false))

(fn `UserConstructionScript`
  (`parent.UserConstructionScript`)
  (set `self.WTimer` (/ (`self.WCooldown`) 2.0))
  (set `self.RTimer` (/ (`self.RCooldown`) 3.0)))