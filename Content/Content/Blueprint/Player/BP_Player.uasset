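; Player character Blueprint on a C++ parent, handling lock-on, melee and Q-spell montages, parry and block.
; Tick projects the lock widget onto the locked enemy, hiding it beyond range, while the mouse wheel retargets sideways relative to the camera.
; Montage events play named sections, with a delayed QIndex reset for the Q spell, and damage derives from the current animation's name.
; Collisions use a frontal-angle check to resolve parries and blocks.
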(event `self.ReceiveTick`
  (params (DeltaSeconds :type "Float (single-precision)"))
  ;[1 1 1] Event Tick
  (`parent.ReceiveTick` DeltaSeconds)
  (bind _targetlock (`self.TargetLock`)
    (:`then`
      (bind _asenemy (cast `Enemy` _targetlock))
      (`self.KeepTargetCentered` _asenemy))
    (:`else`)))

(event `self.ReceiveBeginPlay`
  (bind _returnvalue (`GameplayStatics.GetPlayerController` 0))
  (`parent.ReceiveBeginPlay`)
  ;[1 1 1] Widgets
  ;;[0 0 0] Lock
  (bind _returnvalue_2 (`|CreateWidget` "/Game/Content/UserWidget/Lock/UW_Lock.UW_Lock_C" _returnvalue))
  (`UserWidget.AddToViewport` _returnvalue_2 0)
  (`Widget.SetVisibility` _returnvalue_2 "Hidden")
  (set `self.LockWidget` _returnvalue_2)
  ;;[0 0 0] PlayerQ
  (bind _returnvalue_3 (`|CreateWidget` "/Game/Content/UserWidget/PlayerQ_Health/UW_PlayerQ_Health.UW_PlayerQ_Health_C" _returnvalue))
  (`UserWidget.AddToViewport` _returnvalue_3 0))

(event `self.MontageStartingSectionRandom`
  (params (Montage :type "AnimMontage Object Reference") (name :type String))
  ;[1 1 1] Cpp function play random section from a montage
  (`|PlayMontage` (`self.Mesh`) Montage 1.0 0.0 (`KismetStringLibrary.Conv_StringToName` name)
    (:`OnNotifyBegin`
      (`self.StopAnimMontage` Montage))))

(event `self.MontageQSpell`
  (params (Montage :type "AnimMontage Object Reference") (name :type String))
  ;[1 1 1] Cpp function play q montage
  (`|PlayMontage` (`self.Mesh`) Montage 1.0 0.0 (`KismetStringLibrary.Conv_StringToName` name)
    (:`then`
      (`/Engine/EditorBlueprintResources/StandardMacros.DoOnce` false :!label _label
        (:`Completed`
          (`KismetSystemLibrary.Delay` (`self.QCooldown`))
          (set `self.QIndex` 0)
          (goto _label :!via `Reset`))))
    (:`OnNotifyBegin`
      (`self.StopAnimMontage` Montage))))

(event `EnhancedInput|/Game/Content/Inputs/Lock`
  (params (ActionValue :type Boolean) (ElapsedSeconds :type "Float (double-precision)") (TriggeredSeconds :type "Float (double-precision)") (InputAction :type "InputAction Object Reference" :default "/Game/Content/Inputs/Lock.Lock"))
  ;[1 1 1] Lock
  ;;[0 0 0] Unlock A Target
  (:`Started`
    (`/Engine/EditorBlueprintResources/StandardMacros.FlipFlop`
      (:`B`
        (`Widget.SetVisibility` (`self.LockWidget`) "Hidden")))))

(event `Key|MouseScrollDown`
  (params (Key :type "Key Structure"))
  (bind _returnvalue (`self.K2_GetActorLocation` (`self.TargetLock`)))
  ;[1 1 1] Lock
  ;;[0 0 0] Lock to the left
  (:`Pressed`
    (`self.LockTarget` _returnvalue (+ _returnvalue (* (`KismetMathLibrary.NegateVector` (`KismetMathLibrary.GetRightVector` (`SceneComponent.K2_GetComponentRotation` (`self.Camera`)))) 500.0)))))

(event `Key|MouseScrollUp`
  (params (Key :type "Key Structure"))
  (bind _returnvalue (`self.K2_GetActorLocation` (`self.TargetLock`)))
  ;[1 1 1] Lock
  ;;[0 0 0] Lock to the right
  (:`Pressed`
    (`self.LockTarget` _returnvalue (+ _returnvalue (* (`KismetMathLibrary.GetRightVector` (`SceneComponent.K2_GetComponentRotation` (`self.Camera`))) 500.0)))))

(event `KeepTargetCentered`
  (params (`Target Hit` :type "Enemy Object Reference"))
  (bind _returnvalue (`self.K2_GetActorLocation` `Target Hit`))
  (bind _lockwidget (`self.LockWidget`))
  ;[1 1 1] Lock
  ;;[0 0 0] Keep target centered
  (if (<= (`EntityBase.Health` `Target Hit`) 0.0)
    _
    (elif (> (`KismetMathLibrary.Vector_Distance` (`self.K2_GetActorLocation`) _returnvalue) (`self.MaxDistanceKeepLock`))
      (`Widget.SetVisibility` _lockwidget "Hidden")
      (else
        (`Widget.SetVisibility` _lockwidget "Visible")
        (set `Widget.RenderTransform` (make `WidgetTransform` (`WidgetLayoutLibrary.ProjectWorldLocationToWidgetPosition` (`GameplayStatics.GetPlayerController` 0) _returnvalue true) (1.0 1.0) (2.0 0.0)) _lockwidget)))))

(fn `GetCurrentAnimationDamage`
  (returns (ReturnValue :type "Float (single-precision)"))
  (bind _returnvalue (`KismetStringLibrary.Conv_NameToString` (`self.GetCurrentAnimation`)))
  (if (`KismetStringLibrary.Contains` _returnvalue "Q")
    (return (`self.QDamage_0`))
    (elif (`KismetStringLibrary.Contains` _returnvalue "Attack")
      (return (`self.AttackDamage`))
      (else
        (return 0.0)))))

(fn `OnReceiveCollision`
  (params (OverlappedActor :type "Actor Object Reference") (OtherActor :type "Actor Object Reference"))
  (returns (ReturnValue :type Boolean))
  (bind _returnvalue (< (`KismetMathLibrary.Abs` (- (`KismetMathLibrary.DegAcos` (`KismetMathLibrary.Dot_VectorVector` (`self.GetActorForwardVector`) (`KismetMathLibrary.Normal` (- (`self.K2_GetActorLocation`) (`self.K2_GetActorLocation` OtherActor))))) 180.0)) 45.0))
  (bind _asenemy (cast `Enemy` OtherActor))
  (if (and (`self.IsParryActive`) _returnvalue)
    (`Enemy.OnAttackParried` _asenemy self)
    (`GameplayStatics.PlaySound2D` "/Game/Content/Sounds/Player/Parry.Parry" 1.0 1.0 0.0 null null)
    (else
      (return (not (and _returnvalue (`self.IsBlock`)))))))

(fn `UserConstructionScript`
  (`parent.UserConstructionScript`))