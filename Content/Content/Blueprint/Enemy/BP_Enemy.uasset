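; Enemy Blueprint that shows its health on a widget bar and reports how much damage its current animation deals.
; Each Tick fills the WB_HealthBar from Health over MaxHealth and rotates the widget component to face the player camera.
; GetCurrentAnimationDamage infers damage from the animation name, returning a fixed amount when it contains "Attack" and zero otherwise.
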(event `self.ReceiveTick`
  (params (DeltaSeconds :type "Float (single-precision)"))
  (bind _healthbarwidget (`self.HealthBarWidget`))
  (bind _aswb_health_bar (cast `/Game/Content/Blueprint/UI/WB_HealthBar` (`WidgetComponent.GetWidget` (`self.HealthBarWidget`))))
  (`ProgressBar.SetPercent` (`/Game/Content/Blueprint/UI/WB_HealthBar.HealthBar` _aswb_health_bar) (/ (`self.Health`) (`self.MaxHealth`)))
  (`SceneComponent.K2_SetWorldRotation` _healthbarwidget (`KismetMathLibrary.FindLookAtRotation` (`SceneComponent.K2_GetComponentLocation` _healthbarwidget) (`SceneComponent.K2_GetComponentLocation` (`PlayerCameraManager.TransformComponent` (`GameplayStatics.GetPlayerCameraManager` 0)))) false false))

(fn `GetCurrentAnimationDamage`
  (returns (ReturnValue :type "Float (single-precision)"))
  (if (`KismetStringLibrary.Contains` (`KismetStringLibrary.Conv_NameToString` (`self.GetCurrentAnimation`)) "Attack")
    (return 1.0)
    (else
      (return 0.0))))

(fn `UserConstructionScript`
  (`parent.UserConstructionScript`))